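; WandsPC is a player controller that spawns a wand for its VR pawn when play begins.
; On BeginPlay, only on the authority, it casts the controlled pawn to WandsPawnCharacter and spawns a Wand at the left motion controller's world location and rotation, with itself as owner.
; The wand is not attached or stored here, and a failed cast only prints a message.
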(event EventBeginPlay
  (bind _self self)
  (|CallParentFunction)
  (Networking|SwitchHasAuthority
    (:Authority
      (bind _aswands_pawn_character (Utilities|Casting|CastToWandsPawnCharacter (Pawn|GetControlledPawn _self))
        (:then
          (Game|SpawnActorfromClass "/Game/WandsCPP/Blueprints/Wand.Wand_C" (Math|Transform|MakeTransform (.location (Transformation|GetWorldTransform (Variables|/Script/VRExpansionPlugin.VRBaseCharacter|GetLeftMotionController _aswands_pawn_character))) (.rotation (Transformation|GetWorldTransform (Variables|/Script/VRExpansionPlugin.VRBaseCharacter|GetLeftMotionController _aswands_pawn_character))) "1,1,1") "Undefined" _self 0))
        (:CastFailed
          (Development|PrintString "Cast Failed"))))))

(fn ConstructionScript
  (|CallParentFunction))