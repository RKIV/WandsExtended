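; VR wand actor that, while gripped, turns touches on body points into a cast vector and spawns fireballs.
; While in use, its server-side tick records the character component overlapping the tip.
; Ending an overlap writes that shoulder or hip's index into the vector.
; The server spawns a fireball at the tip whenever per-frame tip movement is below a threshold and the vector is not unset.
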(event Custom|SetIsCasting
  (params (IsCasting :type Boolean))
  (Variables|Casting|SetIsCasting IsCasting))

(event Custom|AddToCastVectorServer
  (params (Component%20Name :type String))
  (CallFunction|AddtoCastVector Component%20Name))

(event Custom|CastSpellServer
  (Class|GrippableStaticMeshActor|IsHeld)
  (Game|SpawnActorfromClass "/Game/WandsCPP/Blueprints/Spells/FireballBP.FireballBP_C" (Transformation|GetWorldTransform (Variables|Default|GetWandTip)) "Undefined" 0 0))

(event EventOnGrip
  (params (GrippingController :type Grip%20Motion%20Controller%20Component%20Object%20Reference) (GripInformation :type BP%20Actor%20Grip%20Information%20Structure%20%28by%20ref%29))
  (Actor|Tick|SetActorTickEnabled true)
  (GameplayTags|AddGameplayTag (Variables|Default|GetGameplayTags) "(TagName=\"DropType.OnSideGrip\")" :!class /Script/GameplayTags.BlueprintGameplayTagLibrary))

(event EventTick
  (params (DeltaSeconds :type Float%20%28single-precision%29))
  (bind _wandtip (Variables|Default|GetWandTip))
  (bind _wandtip_2 (Variables|Default|GetWandTip))
  (bind _returnvalue (Transformation|GetWorldLocation _wandtip_2))
  (if (Utilities|Enum|Equal(Enum) (Networking|GetLocalRole) "ROLE_Authority")
    (Utilities|FlowControl|Sequence
      (:then_0
        (if (Variables|Casting|GetIsCasting)
          (if (> (Utilities|Array|Length (Collision|GetOverlappingActors _wandtip "/Game/WandsCPP/Blueprints/WandsPawnCharacter.WandsPawnCharacter_C" :!class /Script/Engine.PrimitiveComponent)) 0)
            (bind _array_element (Utilities|Array|ForEachLoopwithBreak (Class|PrimitiveComponent|GetOverlappingComponents _wandtip) :!label _label)
              (:LoopBody
                (Development|PrintString (Utilities|GetObjectName _array_element))
                (Variables|Casting|SetPotentialCastComponent (Utilities|GetObjectName _array_element))
                (goto _label Break))))
          (else
            (Development|PrintString "not casting"))))
      (:then_1
        (Variables|Velocity|SetTipVelocity (- _returnvalue (Variables|Velocity|GetPreviousLocation)))
        (Variables|Velocity|SetPreviousLocation _returnvalue))
      (:then_2
        (if (and (< (Math|Vector|VectorLength (Variables|Velocity|GetTipVelocity)) 2e+02) (Class|KismetMathLibrary|NotEqualExactlyVectorVector "-1.000000,-1.000000,-1.000000" (Variables|Casting|GetCast_Vector)))
          (CallFunction|CastSpellServer))))))

(event EventOnEndUsed
  (CallFunction|SetIsCasting false))

(event EventOnUsed
  (CallFunction|SetIsCasting true))

(event Collision|EventActorEndOverlap
  (params (OtherActor :type Actor%20Object%20Reference))
  (bind _potentialcastcomponent (Variables|Casting|GetPotentialCastComponent))
  (if (Utilities|Enum|NotEqual(Enum) "NULL" _potentialcastcomponent)
    (CallFunction|AddtoCastVectorServer _potentialcastcomponent)))

(event EventOnGripRelease
  (params (ReleasingController :type Grip%20Motion%20Controller%20Component%20Object%20Reference) (GripInformation :type BP%20Actor%20Grip%20Information%20Structure%20%28by%20ref%29) (bWasSocketed :type Boolean))
  (Actor|Tick|SetActorTickEnabled false))

(fn ConstructionScript)

(fn AddtoCastVector
  (params (String :type String))
  (switch string String
    (:Default
      (Variables|Temp|SetBodyPartIndex 0 :!label _label))
    (:left_shoulder
      (goto _label))
    (:right_shoulder
      (Variables|Temp|SetBodyPartIndex 1))
    (:left_hip
      (Variables|Temp|SetBodyPartIndex 2))
    (:rihgt_hip
      (Variables|Temp|SetBodyPartIndex 3)))
  (if (!= (.x (Variables|Casting|GetCast_Vector)) -1.0)
    (Variables|Casting|SetCast_Vector (Math|Vector|MakeVector (Math|Conversions|ToFloat(Integer) (Variables|Temp|GetBodyPartIndex)) (.y (Variables|Casting|GetCast_Vector)) (.z (Variables|Casting|GetCast_Vector))))
    (else
      (Variables|Casting|SetCast_Vector (Math|Vector|MakeVector (.x (Variables|Casting|GetCast_Vector)) (Math|Conversions|ToFloat(Integer) (Variables|Temp|GetBodyPartIndex)) (.z (Variables|Casting|GetCast_Vector)))))))